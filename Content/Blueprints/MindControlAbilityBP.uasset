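; Mind control projectile that temporarily turns an enemy Attacker into a friendly Defender.
; Tick moves it along its forward vector and destroys it after a short lifetime if it hits nothing.
; Overlapping a living Attacker stops it, plays a sound, destroys that Attacker and its weapon, and spawns an idle Defender there.
; After a timer, it replaces the Defender with a new seeking Attacker at the saved original transform, then destroys itself.
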(event `self.ReceiveActorBeginOverlap`
  (params (OtherActor :type "Actor Object Reference"))
  (bind _locationdef (`self.LocationDef`))
  (if (not (`self.isHitting`))
    (bind _asattacker (cast `/Game/Characters/Attacker` OtherActor))
    (`/Engine/EditorBlueprintResources/StandardMacros.IsValid` OtherActor
      (:`Is Valid`
        (set `self.LocationDef` (`self.GetTransform` _asattacker))
        (if (`|EnumInequality` (`BaseCharacter.state` _asattacker) "Dead")
          (set `self.isHitting` true)
          (set `self.isChanged` true)
          (set `self.speed` 0.0)
          (`GameplayStatics.PlaySoundAtLocation` null "/Game/Weapons/Sound/GrenadeLauncher/Wavs/GL_Explosion03.GL_Explosion03" (`self.K2_GetActorLocation` OtherActor))
          (`self.K2_DestroyActor` (`BaseCharacter.CurrentWeapon` _asattacker))
          (`self.K2_DestroyActor` _asattacker)
          (`self.K2_SetActorLocation` (`KismetMathLibrary.MakeVector` (.x (.location _locationdef)) (.y (.location _locationdef)) (+ (.z (.location _locationdef)) 200.0)))
          (bind _returnvalue (`|SpawnActorFromClass` "/Game/Characters/Defender.Defender_C" (`self.LocationDef`) "Undefined" "OverrideRootScale"))
          (set `BaseCharacter.state` "Idle" _returnvalue)
          (set `self.tempDef` _returnvalue))))))

(event `self.ReceiveTick`
  (params (DeltaSeconds :type "Float (single-precision)"))
  (bind _timer (`self.timer`))
  (bind _tempdef (`self.tempDef`))
  (`|ExecutionSequence`
    (:`then_0`
      (if (not (`self.isHitting`))
        (set `self.timer` (+ _timer DeltaSeconds))
        (if (>= _timer 3.0)
          (`self.K2_DestroyActor`))))
    (:`then_1`
      (if (not (`self.isHitting`))
        (`self.K2_SetActorTransform` (`KismetMathLibrary.MakeTransform` (+ (.location (`self.GetTransform`)) (* (`KismetMathLibrary.Normal` (`self.GetActorForwardVector`)) (* (`GameplayStatics.GetWorldDeltaSeconds`) (`self.speed`)))) (.rotation (`self.GetTransform`)) (.scale (`self.GetTransform`))))))
    (:`then_2`
      (if (`self.isChanged`)
        (set `self.changeTimer` (+ (`self.changeTimer`) DeltaSeconds))
        (if (>= (`self.changeTimer`) 5.0)
          (`self.K2_DestroyActor` (`BaseCharacter.CurrentWeapon` _tempdef))
          (`self.K2_DestroyActor` _tempdef)
          (bind _returnvalue (`|SpawnActorFromClass` "/Game/Characters/Attacker.Attacker_C" (`self.LocationDef`) "Undefined" "OverrideRootScale"))
          (set `BaseCharacter.state` "Seeking" _returnvalue)
          (`self.K2_DestroyActor`))))))

(fn `UserConstructionScript`)