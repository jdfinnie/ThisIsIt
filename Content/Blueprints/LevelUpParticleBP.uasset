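; LevelUpParticleBP is an actor that serves as a short-lived level-up effect attached by position to the player.
; Each Tick it moves itself to the first player character's location, without sweeping.
; It accumulates delta time in a timer and destroys itself once two seconds have passed.
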(event `self.ReceiveBeginPlay`)

(event `self.ReceiveActorBeginOverlap`
  (params (OtherActor :type "Actor Object Reference")))

(event `self.ReceiveTick`
  (params (DeltaSeconds :type "Float (single-precision)"))
  (`self.K2_SetActorLocation` (`self.K2_GetActorLocation` (`GameplayStatics.GetPlayerCharacter` 0)))
  (set `self.LevelUpTimer` (+ (`self.LevelUpTimer`) DeltaSeconds))
  (if (>= (`self.LevelUpTimer`) 2.0)
    (set `self.LevelUpTimer` 0.0)
    (`self.K2_DestroyActor`)))

(fn `UserConstructionScript`)