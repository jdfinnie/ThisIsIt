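; LightningShockBP is a lightning projectile that knocks an Attacker into its Idle state on overlap, then destroys itself.
; Tick moves it forward at Speed while IsHitting is false and destroys it once its three-second lifetime timer runs out.
; An unconnected chain holds a timed stun that would return a living Attacker to Seeking, so nothing here restores that state.
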(event `self.ReceiveBeginPlay`)

(event `self.ReceiveActorBeginOverlap`
  (params (OtherActor :type "Actor Object Reference"))
  (bind _asattacker (cast `/Game/Characters/Attacker` OtherActor))
  (set `BaseCharacter.state` "Idle" _asattacker)
  (`self.K2_DestroyActor`))

(event `self.ReceiveTick`
  (params (DeltaSeconds :type "Float (single-precision)"))
  (bind _timer (`self.timer`))
  (`|ExecutionSequence`
    (:`then_0`
      (set `self.timer` (+ _timer DeltaSeconds))
      (if (>= _timer 3.0)
        (`self.K2_DestroyActor`)))
    (:`then_1`
      (if (not (`self.isHitting`))
        (`self.K2_SetActorTransform` (`KismetMathLibrary.MakeTransform` (+ (.location (`self.GetTransform`)) (* (`KismetMathLibrary.Normal` (`self.GetActorForwardVector`)) (* (`GameplayStatics.GetWorldDeltaSeconds`) (`self.speed`)))) (.rotation (`self.GetTransform`)) (.scale (`self.GetTransform`))))))))

(fn `UserConstructionScript`)