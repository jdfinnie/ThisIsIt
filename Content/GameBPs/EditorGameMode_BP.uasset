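; Game mode for a building layout editor that restores and saves placed buildings across level loads.
; On BeginPlay it reads transforms from ThisIsIt_GameInstance_BP, spawns the unique hub plus large, medium and small buildings, and tracks them in per-type arrays.
; SaveLayout writes those actors' current transforms back to the game instance, keeping one transform for the unique building.
; ChangeLevel saves the layout, then opens EditorTest2.
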(event EventBeginPlay
  (bind _asthis_is_it_game_instance_bp (Utilities|Casting|CastToThisIsIt_GameInstance_BP (Game|GetGameInstance))
    (:then
      (Variables|Default|SetInstance _asthis_is_it_game_instance_bp)
      (Utilities|FlowControl|Sequence
        (:then_0
          (CallFunction|SpawnHub))
        (:then_1
          (CallFunction|SpawnLarge))
        (:then_2
          (CallFunction|SpawnMed))
        (:then_3
          (CallFunction|SpawnSmall))))
    (:CastFailed
      (Development|PrintString 0 "no instance"))))

(fn ConstructionScript)

(fn SaveLayout
  (bind _instance (Variables|Default|GetInstance))
  (bind _newlocalvar_0 (LocalVariables|GetNewLocalVar_0))
  ;[1 1 1] clear existing
  (Variables|/Game/GameBPs/ThisIsIt_GameInstance_BP.ThisIsIt_GameInstance_BP_C|SetSmallTransforms (Variables|Default|GetInstance) _newlocalvar_0)
  (Variables|/Game/GameBPs/ThisIsIt_GameInstance_BP.ThisIsIt_GameInstance_BP_C|SetLargeTransforms _instance _newlocalvar_0)
  (Variables|/Game/GameBPs/ThisIsIt_GameInstance_BP.ThisIsIt_GameInstance_BP_C|SetMedTransforms _instance _newlocalvar_0)
  ;[1 1 1] Add local objects
  (for _array_element (Variables|Default|GetSmallBuildings)
    (Utilities|Array|Add (Variables|/Game/GameBPs/ThisIsIt_GameInstance_BP.ThisIsIt_GameInstance_BP_C|GetSmallTransforms (Variables|Default|GetInstance)) (Transformation|GetActorTransform _array_element)))
  (for _array_element_2 (Variables|Default|GetMedBuildings)
    (Utilities|Array|Add (Variables|/Game/GameBPs/ThisIsIt_GameInstance_BP.ThisIsIt_GameInstance_BP_C|GetMedTransforms (Variables|Default|GetInstance)) (Transformation|GetActorTransform _array_element_2)))
  (for _array_element_3 (Variables|Default|GetLargeBuildings)
    (Utilities|Array|Add (Variables|/Game/GameBPs/ThisIsIt_GameInstance_BP.ThisIsIt_GameInstance_BP_C|GetLargeTransforms (Variables|Default|GetInstance)) (Transformation|GetActorTransform _array_element_3)))
  (for _array_element_4 (Variables|Default|GetUniqueBuildings)
    (Variables|/Game/GameBPs/ThisIsIt_GameInstance_BP.ThisIsIt_GameInstance_BP_C|SetUniqueTransform (Variables|Default|GetInstance) (Transformation|GetActorTransform _array_element_4))))

(fn SpawnHub
  (bind _returnvalue (Game|SpawnActorfromClass "/Game/Buildings/Building_BP_Unique.Building_BP_Unique_C" (Variables|/Game/GameBPs/ThisIsIt_GameInstance_BP.ThisIsIt_GameInstance_BP_C|GetUniqueTransform (Variables|Default|GetInstance)) "Undefined" 0 0))
  (Utilities|Array|Add (Variables|Default|GetUniqueBuildings) _returnvalue))

(fn SpawnLarge
  (for _array_element (Variables|/Game/GameBPs/ThisIsIt_GameInstance_BP.ThisIsIt_GameInstance_BP_C|GetLargeTransforms (Variables|Default|GetInstance))
    (bind _returnvalue (Game|SpawnActorfromClass "/Game/Buildings/Building_BP_Large.Building_BP_Large_C" _array_element "Undefined" 0 0))
    (Utilities|Array|Add (Variables|Default|GetLargeBuildings) _returnvalue)))

(fn SpawnMed
  (for _array_element (Variables|/Game/GameBPs/ThisIsIt_GameInstance_BP.ThisIsIt_GameInstance_BP_C|GetMedTransforms (Variables|Default|GetInstance))
    (bind _returnvalue (Game|SpawnActorfromClass "/Game/Buildings/Building_BP_Med.Building_BP_Med_C" _array_element "Undefined" 0 0))
    (Utilities|Array|Add (Variables|Default|GetMedBuildings) _returnvalue)))

(fn SpawnSmall
  (for _array_element (Variables|/Game/GameBPs/ThisIsIt_GameInstance_BP.ThisIsIt_GameInstance_BP_C|GetSmallTransforms (Variables|Default|GetInstance))
    (bind _returnvalue (Game|SpawnActorfromClass "/Game/Buildings/Building_BP_Small.Building_BP_Small_C" _array_element "Undefined" 0 0))
    (Utilities|Array|Add (Variables|Default|GetSmallBuildings) _returnvalue)))

(fn ChangeLevel
  (CallFunction|SaveLayout)
  (Game|OpenLevel(byName) 0 "EditorTest2"))